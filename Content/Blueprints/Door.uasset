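; Keycard-locked door actor that the first-person character can open by holding a key matching the door's Id.
; When interactable, overlapping its box registers it as the player's InteractActor and swaps to an unlockable material if a collected key matches; leaving resets both.
; The Unlock event destroys the door when a passed key matches.
; Non-interactable doors skip registration and clear both card meshes at BeginPlay.
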(event `self.ReceiveBeginPlay`
  (bind _cardmaterial (`self.cardMaterial`))
  (`PrimitiveComponent.SetMaterial` (`self.StaticMesh`) 0 (`self.defaultMaterial`))
  (if (`self.canInteract`)
    (`PrimitiveComponent.SetMaterial` (`self.Card1`) 0 _cardmaterial)
    (`PrimitiveComponent.SetMaterial` (`self.Card2`) 0 _cardmaterial)
    (else
      (`StaticMeshComponent.SetStaticMesh` (`self.Card1`) null)
      (`StaticMeshComponent.SetStaticMesh` (`self.Card2`) null))))

(event `self.Box.OnComponentBeginOverlap`
  (params (OverlappedComponent :type "PrimitiveComponent Object Reference") (OtherActor :type "Actor Object Reference") (OtherComp :type "PrimitiveComponent Object Reference") (OtherBodyIndex :type Integer) (bFromSweep :type Boolean) (SweepResult :type "HitResult Structure (by ref)"))
  (if (`self.canInteract`)
    (bind _asbp_first_person_character (cast `/Game/FirstPerson/Blueprints/BP_FirstPersonCharacter` OtherActor))
    (set `/Game/FirstPerson/Blueprints/BP_FirstPersonCharacter.interactActor` self _asbp_first_person_character)
    (set `self.player` _asbp_first_person_character)
    (`KismetSystemLibrary.PrintString` "Unlock")
    (for _array_element (`/Game/FirstPerson/Blueprints/BP_FirstPersonCharacter.CollectedKeys` (`self.player`))
      (if (== _array_element (`self.id`))
        (`PrimitiveComponent.SetMaterial` (`self.StaticMesh`) 0 (`self.unlockableMaterial`))))))

(event `self.Box.OnComponentEndOverlap`
  (params (OverlappedComponent :type "PrimitiveComponent Object Reference") (OtherActor :type "Actor Object Reference") (OtherComp :type "PrimitiveComponent Object Reference") (OtherBodyIndex :type Integer))
  (bind _asbp_first_person_character (cast `/Game/FirstPerson/Blueprints/BP_FirstPersonCharacter` OtherActor))
  (set `/Game/FirstPerson/Blueprints/BP_FirstPersonCharacter.interactActor` null _asbp_first_person_character)
  (`PrimitiveComponent.SetMaterial` (`self.StaticMesh`) 0 (`self.defaultMaterial`)))

(event `Unlock`
  (params (keyID :type "Array of Integer"))
  (for _array_element keyID
    (if (== _array_element (`self.id`))
      (`self.K2_DestroyActor`))))

(fn `UserConstructionScript`)