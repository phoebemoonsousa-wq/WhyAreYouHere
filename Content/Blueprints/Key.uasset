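; Key is a collectible pickup that the first-person character collects to gain a key Id.
; Its sphere overlap registers the key as the character's InteractActor while CanInteract is set, and clears that reference on exit, printing debug prompts.
; The Interacted event adds the Id to the player's CollectedKeys, clears the interaction reference and destroys the key.
; A configurable material is applied to the mesh at BeginPlay.
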(event `self.ReceiveBeginPlay`
  (`PrimitiveComponent.SetMaterial` (`self.StaticMesh`) 0 (`self.material`)))

(event `self.Sphere.OnComponentBeginOverlap`
  (params (OverlappedComponent :type "PrimitiveComponent Object Reference") (OtherActor :type "Actor Object Reference") (OtherComp :type "PrimitiveComponent Object Reference") (OtherBodyIndex :type Integer) (bFromSweep :type Boolean) (SweepResult :type "HitResult Structure (by ref)"))
  (if (`self.canInteract`)
    (bind _asbp_first_person_character (cast `/Game/FirstPerson/Blueprints/BP_FirstPersonCharacter` OtherActor))
    (set `/Game/FirstPerson/Blueprints/BP_FirstPersonCharacter.interactActor` self _asbp_first_person_character)
    (set `self.player` _asbp_first_person_character)
    (`KismetSystemLibrary.PrintString` "Press E")))

(event `self.Sphere.OnComponentEndOverlap`
  (params (OverlappedComponent :type "PrimitiveComponent Object Reference") (OtherActor :type "Actor Object Reference") (OtherComp :type "PrimitiveComponent Object Reference") (OtherBodyIndex :type Integer))
  (bind _asbp_first_person_character (cast `/Game/FirstPerson/Blueprints/BP_FirstPersonCharacter` OtherActor))
  (set `/Game/FirstPerson/Blueprints/BP_FirstPersonCharacter.interactActor` null _asbp_first_person_character)
  (`KismetSystemLibrary.PrintString` "Left"))

(event `Interacted`
  (bind _player (`self.player`))
  (`KismetSystemLibrary.PrintString` "Collected")
  (`KismetArrayLibrary.Array_Add` (`/Game/FirstPerson/Blueprints/BP_FirstPersonCharacter.CollectedKeys` _player) (`self.id`))
  (set `/Game/FirstPerson/Blueprints/BP_FirstPersonCharacter.interactActor` null _player)
  (`self.K2_DestroyActor`))

(fn `UserConstructionScript`)