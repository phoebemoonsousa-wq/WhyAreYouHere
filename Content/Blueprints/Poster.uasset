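; Poster is an interactable that gates a card-matching minigame behind a collected key and removes a linked door when won.
; Sphere overlap registers it as the first-person character's InteractActor and shows a prompt.
; CardGame checks the player's CollectedKeys for its Id, then opens the CardMatchingGame widget with movement locked and UI-only input, or prints a missing-piece message.
; WonGame destroys DoorRef.
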(event `self.Sphere.OnComponentBeginOverlap`
  (params (OverlappedComponent :type "PrimitiveComponent Object Reference") (OtherActor :type "Actor Object Reference") (OtherComp :type "PrimitiveComponent Object Reference") (OtherBodyIndex :type Integer) (bFromSweep :type Boolean) (SweepResult :type "HitResult Structure (by ref)"))
  (if (`self.canInteract`)
    (bind _asbp_first_person_character (cast `/Game/FirstPerson/Blueprints/BP_FirstPersonCharacter` OtherActor))
    (set `/Game/FirstPerson/Blueprints/BP_FirstPersonCharacter.interactActor` self _asbp_first_person_character)
    (set `self.player` _asbp_first_person_character)
    (`KismetSystemLibrary.PrintString` "Press E")))

(event `CardGame`
  (bind _returnvalue (`GameplayStatics.GetPlayerController` 0))
  (bind _collectedkeys (`/Game/FirstPerson/Blueprints/BP_FirstPersonCharacter.CollectedKeys` (`self.player`)))
  (if (`KismetArrayLibrary.Array_Contains` _collectedkeys (`self.id`))
    (for _array_element _collectedkeys
      (if (== _array_element (`self.id`))
        (bind _returnvalue_2 (`|CreateWidget` "/Game/Blueprints/CardMatchingGame.CardMatchingGame_C" (`GameplayStatics.GetPlayerController` 0)))
        (`UserWidget.AddToViewport` _returnvalue_2 0)
        (set `/Game/Blueprints/CardMatchingGame.poster` self _returnvalue_2)
        (set `/Game/FirstPerson/Blueprints/BP_FirstPersonCharacter.canMove` false (`self.player`))
        (`WidgetBlueprintLibrary.SetInputMode_UIOnlyEx` _returnvalue _returnvalue_2)
        (set `PlayerController.bShowMouseCursor` true _returnvalue)))
    (else
      (`KismetSystemLibrary.PrintString` "You are missing a piece..." true true (struct :`R` 1.0 :`A` 1.0) 4.0))))

(event `WonGame`
  (`self.K2_DestroyActor` (`self.doorRef`)))

(fn `UserConstructionScript`)